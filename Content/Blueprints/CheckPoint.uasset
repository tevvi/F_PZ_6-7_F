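; CheckPoint is a checkpoint trigger that saves the player's progress when a BP_TopDownCharacter overlaps its Box component.
; On overlap it creates a fresh SaveBlueprint save object, fills its inventory profile from the character's inventory widget slots and stores the character's location.
; It then saves synchronously to the slot name and index held by that object, with debug prints for the overlap and the save result.
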(event OnComponentBeginOverlap(Box)
  (params (OverlappedComponent :type Primitive%20Component%20Object%20Reference) (OtherActor :type Actor%20Object%20Reference) (OtherComp :type Primitive%20Component%20Object%20Reference) (OtherBodyIndex :type Integer) (bFromSweep :type Boolean) (SweepResult :type Hit%20Result%20Structure%20%28by%20ref%29))
  (Development|PrintString "Hello")
  (bind _asbp_top_down_character (Utilities|Casting|CastToBP_TopDownCharacter OtherActor))
  (bind _returnvalue (SaveGame|CreateSaveGameObject "/Game/Blueprints/SaveBlueprint.SaveBlueprint_C"))
  (bind _output_get (Variables|Default|SetSaveInstance _returnvalue))
  (Utilities|Array|Clear (Variables|/Game/Blueprints/SaveBlueprint.SaveBlueprint_C|GetInventoryProfile _output_get))
  (for _array_element (Variables|/Script/Inventory.InventoryWidget|GetSlots (Variables|/Game/Blueprints/BP_TopDownCharacter.BP_TopDownCharacter_C|GetInventoryWIdget _asbp_top_down_character))
    (Utilities|Array|Add (Variables|/Game/Blueprints/SaveBlueprint.SaveBlueprint_C|GetInventoryProfile _output_get) (Variables|/Script/Inventory.SlotWidget|GetItem _array_element)))
  (Variables|/Game/Blueprints/SaveBlueprint.SaveBlueprint_C|SetActorLoc _returnvalue (Transformation|GetActorLocation _asbp_top_down_character))
  (bind _returnvalue_2 (SaveGame|SaveGametoSlot _output_get (Variables|/Game/Blueprints/SaveBlueprint.SaveBlueprint_C|GetSlotName _output_get) (Variables|/Game/Blueprints/SaveBlueprint.SaveBlueprint_C|GetSlotIndex _output_get)))
  (if _returnvalue_2
    (Development|PrintString "yes")
    (else
      (Development|PrintString "no"))))

(event EventBeginPlay)

(event Collision|EventActorBeginOverlap
  (params (OtherActor :type Actor%20Object%20Reference)))

(event EventTick
  (params (DeltaSeconds :type Float%20%28single-precision%29)))

(fn ConstructionScript)