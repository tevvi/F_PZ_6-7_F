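; A game instance Blueprint that restores saved inventory and an actor location when the game starts.
; On Init it checks whether the InvLoad save slot exists, loads it and casts it to SaveBlueprint.
; It copies the saved InventoryProfile and ActorLoc into its own Items and VectorVar variables; it does no saving and does not move any actor itself.
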(event EventInit
  (bind _returnvalue (SaveGame|DoesSaveGameExist (Variables|Default|GetInvLoad) (Variables|Default|GetIndex)))
  (if _returnvalue
    (bind _returnvalue_2 (SaveGame|LoadGamefromSlot (Variables|Default|GetInvLoad) (Variables|Default|GetIndex)))
    (bind _assave_blueprint (Utilities|Casting|CastToSaveBlueprint _returnvalue_2))
    (Variables|Default|SetItems (Variables|/Game/Blueprints/SaveBlueprint.SaveBlueprint_C|GetInventoryProfile _assave_blueprint))
    (Variables|Default|SetVectorVar (Variables|/Game/Blueprints/SaveBlueprint.SaveBlueprint_C|GetActorLoc _assave_blueprint))))